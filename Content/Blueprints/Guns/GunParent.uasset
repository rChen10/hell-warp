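; Base gun Blueprint for an FPS character, handling single-shot and automatic SMG firing with sound.
; SMG fire runs on a timer that checks the owner's ammo, while other guns fire once without that check.
; FireBullet reaches the owner through the parent actor, deducts ammo and, for hitscan guns, line-traces from the camera.
; Hits damage BP_FPSOpponent, update its health widget and destroy it when health runs out.
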(event `StartShooting`
  (params (`Is SMG` :type Boolean))
  (set `self.isFiring` true)
  (if `Is SMG`
    (`KismetSystemLibrary.K2_SetTimerDelegate` (delegate `KeepShooting`) 0.1 (`self.isFiring`))
    (else
      (`self.FireBullet`)
      (if (== (`self.AmmoSize`) 0)
        (`AddComponent|NODE_AddAudioComponent-0`)
        (`GameplayStatics.PlaySound2D` "/Game/Sounds/PistolShotNoise.PistolShotNoise" 1.0 1.0 0.0 null null)
        (elif (== (`self.AmmoSize`) 4)
          _)))))

(event `StopShooting`
  (set `self.isFiring` false))

(event `KeepShooting`
  (bind _asbp_fpscharacter (cast `/Game/Blueprints/BP_FPSCharacter` (`self.GetParentActor`)))
  (if (and (> (`/Game/Blueprints/BP_FPSCharacter.CurrentAmmo` _asbp_fpscharacter) 0) (`self.isFiring`))
    (`self.FireBullet`)
    (`AddComponent|NODE_AddAudioComponent-2`)
    (`GameplayStatics.PlaySound2D` "/Game/Sounds/AKShotQue.AKShotQue" 1.0 1.0 0.0 null null)))

(fn `FireBullet`
  (bind _asbp_fpscharacter (cast `/Game/Blueprints/BP_FPSCharacter` (`self.GetParentActor`)))
  (set `/Game/Blueprints/BP_FPSCharacter.CurrentAmmo` (- (`/Game/Blueprints/BP_FPSCharacter.CurrentAmmo` _asbp_fpscharacter) (`self.AmmoSize`)) _asbp_fpscharacter)
  (if (`self.isHitscan`)
    (bind _asfpscharacter (cast `FPSCharacter` (`self.GetParentActor`)))
    (bind _fpscameracomponent (`FPSCharacter.FPSCameraComponent` _asfpscharacter))
    (bind _returnvalue (`SceneComponent.K2_GetComponentLocation` _fpscameracomponent))
    (bind _outhit (`KismetSystemLibrary.LineTraceSingle` _returnvalue (+ (* (`KismetMathLibrary.GetForwardVector` (`SceneComponent.K2_GetComponentRotation` _fpscameracomponent)) 2000.0) _returnvalue) "TraceTypeQuery1"))
    (`|ExecutionSequence`
      (:`then_0`
        (bind (_bblockinghit _binitialoverlap _time _distance _location _impactpoint _normal _impactnormal _physmat _hitactor) (`GameplayStatics.BreakHitResult` _outhit))
        (`KismetSystemLibrary.PrintString` (`KismetSystemLibrary.GetDisplayName` _hitactor)))
      (:`then_1`
        (bind _asbp_fpsopponent (cast `/Game/Blueprints/Enemies/BP_FPSOpponent` _hitactor))
        (bind _returnvalue_2 (- (`/Game/Blueprints/Enemies/BP_FPSOpponent.Health` _asbp_fpsopponent) (`KismetMathLibrary.FTrunc` (* (`FPSCharacter.Damage` _asfpscharacter) 10.0))))
        (set `/Game/Blueprints/Enemies/BP_EnemyHealth.Health` (`KismetMathLibrary.Conv_IntToDouble` _returnvalue_2) (`/Game/Blueprints/Enemies/BP_FPSOpponent.Health Widget REF` _asbp_fpsopponent))
        (if (< _returnvalue_2 1)
          (`/Game/Blueprints/Enemies/BP_FPSOpponent.Die` _asbp_fpsopponent)
          (`self.K2_DestroyActor` _asbp_fpsopponent)
          (else
            (bind _output_get (set `/Game/Blueprints/Enemies/BP_FPSOpponent.Health` _returnvalue_2 _asbp_fpsopponent))
            (`KismetSystemLibrary.PrintString` (`KismetStringLibrary.BuildString_Int` "" "" _output_get))))))))

(fn `UserConstructionScript`
  (`SceneComponent.K2_AttachToComponent` (`self.Guns`) null "None" "SnapToTarget" "SnapToTarget" "SnapToTarget" true))