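; GunParent is a gun Blueprint, apparently a base class, that expects an FPSCharacter as its parent actor and fires when StartShooting is called.
; Each call fires once: if IsHitscan, FireBullet line-traces forward from the character's camera; non-hitscan firing does nothing.
; Hits on BP_FPSOpponent deal fixed damage, update its health widget, and enable mesh physics simulation on a lethal hit, without storing that final Health.
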(event `StartShooting`
  (set `self.isFiring` true)
  (`self.FireBullet`))

(event `StopShooting`
  (set `self.isFiring` false))

(fn `FireBullet`
  (if (`self.isHitscan`)
    (bind _asfpscharacter (cast `FPSCharacter` (`self.GetParentActor`)))
    (bind _fpscameracomponent (`FPSCharacter.FPSCameraComponent` _asfpscharacter))
    (bind _returnvalue (`SceneComponent.K2_GetComponentLocation` _fpscameracomponent))
    (bind _outhit (`KismetSystemLibrary.LineTraceSingle` _returnvalue (+ (* (`KismetMathLibrary.GetForwardVector` (`SceneComponent.K2_GetComponentRotation` _fpscameracomponent)) 2000.0) _returnvalue) "TraceTypeQuery1"))
    (`|ExecutionSequence`
      (:`then_0`
        (bind (_bblockinghit _binitialoverlap _time _distance _location _impactpoint _normal _impactnormal _physmat _hitactor) (`GameplayStatics.BreakHitResult` _outhit))
        (`KismetSystemLibrary.PrintString` (`KismetSystemLibrary.GetDisplayName` _hitactor)))
      (:`then_1`
        (bind _asbp_fpsopponent (cast `/Game/Blueprints/BP_FPSOpponent` _hitactor))
        (bind _returnvalue_2 (- (`/Game/Blueprints/BP_FPSOpponent.Health` _asbp_fpsopponent) 10))
        (set `/Game/Blueprints/BP_EnemyHealth.Health` (`KismetMathLibrary.Conv_IntToDouble` _returnvalue_2) (`/Game/Blueprints/BP_FPSOpponent.Health Widget REF` _asbp_fpsopponent))
        (if (< _returnvalue_2 1)
          (`PrimitiveComponent.SetSimulatePhysics` (`Character.Mesh` _asbp_fpsopponent) true)
          (else
            (bind _output_get (set `/Game/Blueprints/BP_FPSOpponent.Health` _returnvalue_2 _asbp_fpsopponent))
            (`KismetSystemLibrary.PrintString` (`KismetStringLibrary.BuildString_Int` "" "" _output_get))))))))

(fn `UserConstructionScript`
  (`SceneComponent.K2_AttachToComponent` (`self.Guns`) null "None" "SnapToTarget" "SnapToTarget" "SnapToTarget" true))