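; Base Blueprint for pickup drops that the player character collects by walking into them.
; An overlap with BP_FPSCharacter calls Pickup and then destroys the drop.
; Pickup only prints a placeholder string here, apparently meant for child classes to override.
; Tick spins the root component around yaw at a steady, frame-rate-independent rate.
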(event `self.ReceiveActorBeginOverlap`
  (params (OtherActor :type "Actor Object Reference"))
  (cast `/Game/Blueprints/BP_FPSCharacter` OtherActor)
  (`self.Pickup`)
  (`self.K2_DestroyActor`))

(event `self.ReceiveTick`
  (params (DeltaSeconds :type "Float (single-precision)"))
  (`SceneComponent.K2_AddRelativeRotation` (`self.DefaultSceneRoot`) (`KismetMathLibrary.MakeRotator` 0.0 0.0 (* DeltaSeconds 100.0)) false false))

(fn `Pickup`
  (`KismetSystemLibrary.PrintString` "Drop Parent Class"))

(fn `UserConstructionScript`)