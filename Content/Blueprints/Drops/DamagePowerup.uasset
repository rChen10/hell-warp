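; DamagePowerup is a drop that permanently raises the player's damage when picked up.
; Its Pickup function casts player character 0 to BP_FPSCharacter and increments that character's Damage variable by one.
; The event graph holds only disabled default events, so whatever triggers Pickup lies outside this graph.
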(fn `Pickup`
  (bind _asbp_fpscharacter (cast `/Game/Blueprints/BP_FPSCharacter` (`GameplayStatics.GetPlayerCharacter` 0)))
  (set `/Game/Blueprints/BP_FPSCharacter.Damage` (+ (`/Game/Blueprints/BP_FPSCharacter.Damage` _asbp_fpscharacter) 1) _asbp_fpscharacter))

(fn `UserConstructionScript`
  (`parent.UserConstructionScript`))