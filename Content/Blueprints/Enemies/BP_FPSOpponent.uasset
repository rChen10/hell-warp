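; BP_FPSOpponent is an enemy with a health widget, a timed attack state and a powerup drop.
; BeginPlay sets walk speed and caches the player and health widget references.
; Its sphere toggles the widget as the player enters or leaves; entering at zero health or below instead spawns a health powerup at a nearby reachable point and destroys the enemy.
; Attack sets AttackType, which a short timer resets.
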(event `self.ReceiveBeginPlay`
  (set `self.Drop Ref` "/Game/Blueprints/Drops/Heart/HealthPowerup.HealthPowerup_C")
  (set `CharacterMovementComponent.MaxWalkSpeed` 200.0 (`self.CharacterMovement`))
  (bind _asfpscharacter (cast `FPSCharacter` (`GameplayStatics.GetPlayerCharacter` 0)))
  (set `self.Char Ref` _asfpscharacter)
  (bind _asbp_enemy_health (cast `/Game/Blueprints/Enemies/BP_EnemyHealth` (`WidgetComponent.GetUserWidgetObject` (`self.Widget`))))
  (set `self.Health Widget REF` _asbp_enemy_health))

(event `self.ReceiveTick`
  (params (DeltaSeconds :type "Float (single-precision)")))

(event `self.Sphere.OnComponentBeginOverlap`
  (params (OverlappedComponent :type "PrimitiveComponent Object Reference") (OtherActor :type "Actor Object Reference") (OtherComp :type "PrimitiveComponent Object Reference") (OtherBodyIndex :type Integer) (bFromSweep :type Boolean) (SweepResult :type "HitResult Structure (by ref)"))
  (cast `FPSCharacter` OtherActor)
  (if (> (`self.Health`) 0)
    (`SceneComponent.SetVisibility` (`self.Widget`) true false)
    (else
      (`self.Die`)
      (`self.K2_DestroyActor`))))

(event `self.Sphere.OnComponentEndOverlap`
  (params (OverlappedComponent :type "PrimitiveComponent Object Reference") (OtherActor :type "Actor Object Reference") (OtherComp :type "PrimitiveComponent Object Reference") (OtherBodyIndex :type Integer))
  (cast `FPSCharacter` OtherActor)
  (`SceneComponent.SetVisibility` (`self.Widget`) false false))

(event `Attack`
  (set `self.AttackType` 1)
  (`KismetSystemLibrary.K2_SetTimerDelegate` (delegate `Stop Attack`) 0.5))

(event `Stop Attack`
  (set `self.AttackType` 0))

(fn `Die`
  (`|SpawnActorFromClass` (`self.Drop Ref`) (`KismetMathLibrary.MakeTransform` (`NavigationSystemV1.K2_GetRandomReachablePointInRadius` (`self.K2_GetActorLocation`) 100.0 null null) (`KismetMathLibrary.MakeRotator` 0.0 0.0 (`KismetMathLibrary.RandomFloatInRange` 0.0 360.0))) "Undefined" "OverrideRootScale" null null))

(fn `UserConstructionScript`)