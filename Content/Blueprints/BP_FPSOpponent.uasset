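; BP_FPSOpponent is an opponent Blueprint for an FPS game that reveals a widget, used for enemy health, when the player is near.
; BeginPlay caches the FPSCharacter player and the BP_EnemyHealth instance inside its Widget component.
; Sphere overlap events show the widget when an FPSCharacter enters and hide it when one leaves.
; Tick is empty, and a random-chance Jump is left disconnected, so it never runs.
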(event `self.ReceiveBeginPlay`
  (bind _asfpscharacter (cast `FPSCharacter` (`GameplayStatics.GetPlayerCharacter` 0)))
  (set `self.Char Ref` _asfpscharacter)
  (bind _asbp_enemy_health (cast `/Game/Blueprints/BP_EnemyHealth` (`WidgetComponent.GetUserWidgetObject` (`self.Widget`))))
  (set `self.Health Widget REF` _asbp_enemy_health))

(event `self.ReceiveTick`
  (params (DeltaSeconds :type "Float (single-precision)")))

(event `self.Sphere.OnComponentBeginOverlap`
  (params (OverlappedComponent :type "PrimitiveComponent Object Reference") (OtherActor :type "Actor Object Reference") (OtherComp :type "PrimitiveComponent Object Reference") (OtherBodyIndex :type Integer) (bFromSweep :type Boolean) (SweepResult :type "HitResult Structure (by ref)"))
  (cast `FPSCharacter` OtherActor)
  (`SceneComponent.SetVisibility` (`self.Widget`) true false))

(event `self.Sphere.OnComponentEndOverlap`
  (params (OverlappedComponent :type "PrimitiveComponent Object Reference") (OtherActor :type "Actor Object Reference") (OtherComp :type "PrimitiveComponent Object Reference") (OtherBodyIndex :type Integer))
  (cast `FPSCharacter` OtherActor)
  (`SceneComponent.SetVisibility` (`self.Widget`) false false))

(fn `UserConstructionScript`)